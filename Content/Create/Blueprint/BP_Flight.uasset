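; BP_Flight is a player-controlled flying craft that constantly moves along its forward vector and can fire rockets.
; Tick feeds Speed into movement input, and holding Boost raises that value until release.
; Roll and Pitch axes apply clamped, delta-time-scaled local rotations, steering the flight direction without any yaw input.
; The Short action spawns a BP_Rocket at the Arrow component's world transform.
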(event `InputAction|Boost`
  (params (Key :type "Key Structure"))
  (:`Pressed`
    (set `self.Speed` 1.0))
  (:`Released`
    (set `self.Speed` 0.5)))

(event `self.ReceiveTick`
  (params (DeltaSeconds :type "Float (single-precision)"))
  ;[0.04231 0.02122 0.02029 1 15] Movement_Front
  (`self.AddMovementInput` (`self.GetActorForwardVector`) (`self.Speed`)))

(event `InputAction|Short`
  (params (Key :type "Key Structure"))
  (:`Pressed`
    (`|SpawnActorFromClass` "/Game/Create/Blueprint/BP_Rocket.BP_Rocket_C" (`SceneComponent.K2_GetComponentToWorld` (`self.Arrow`)) "AdjustIfPossibleButAlwaysSpawn" "MultiplyWithRoot" null null)))

(event `InputAxis|Roll`
  (params (AxisValue :type "Float (single-precision)"))
  ;[0.02217 0.07819 0.01096 1 15] Movement_Roll
  (`self.K2_AddActorLocalRotation` (`KismetMathLibrary.MakeRotator` (* (`KismetMathLibrary.FClamp` AxisValue -1.0) 50.0 (`GameplayStatics.GetWorldDeltaSeconds`)))))

(event `InputAxis|Pitch`
  (params (AxisValue :type "Float (single-precision)"))
  ;[0.06301 0.1651 0.2664 1 15] Movement_Pitch
  (`self.K2_AddActorLocalRotation` (`KismetMathLibrary.MakeRotator` 0.0 (* (`KismetMathLibrary.FClamp` AxisValue -1.0) 50.0 (`GameplayStatics.GetWorldDeltaSeconds`)))))

(fn `UserConstructionScript`)